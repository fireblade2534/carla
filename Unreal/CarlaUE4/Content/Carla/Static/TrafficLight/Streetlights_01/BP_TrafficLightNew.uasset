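; Traffic light actor that shows red, yellow or green and relays state changes to car trigger observers.
; Construction script builds meshes from Heads data, grouping each light's dynamic material instance by color.
; BeginPlay wraps each box except TotalVolume in a BPCustomTrigger component bound to overlaps.
; State changes toggle each group's On/Off parameter and notify those triggers; UnifyTriggers destroys every box except TotalVolume.
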(event `Unify Triggers`
  (for _array_element (`self.K2_GetComponentsByClass` "/Script/Engine.BoxComponent")
    (if (not (`KismetStringLibrary.EqualEqual_StrStr` (`KismetSystemLibrary.GetDisplayName` _array_element) "TotalVolume"))
      (`ActorComponent.K2_DestroyComponent` _array_element))))

(event `self.ReceiveBeginPlay`
  (`self.CreateCarObservers`))

(event `self.OnTrafficLightStateChanged`
  (params (TrafficLightState :type "TrafficLightState Structure"))
  (bind (_bred _byellow _bgreen) (break `TrafficLightState` TrafficLightState))
  (`|ExecutionSequence`
    (:`then_0`
      (for _array_element (`self.RedLights`)
        (`MaterialInstanceDynamic.SetScalarParameterValue` _array_element "On/Off" (`KismetMathLibrary.SelectFloat` 1.0 0.0 _bred)))
      (for _array_element_2 (`self.YellowLights`)
        (`MaterialInstanceDynamic.SetScalarParameterValue` _array_element_2 "On/Off" (`KismetMathLibrary.SelectFloat` 1.0 0.0 _byellow)))
      (for _array_element_3 (`self.GreenLights`)
        (`MaterialInstanceDynamic.SetScalarParameterValue` _array_element_3 "On/Off" (`KismetMathLibrary.SelectFloat` 1.0 0.0 _bgreen))))
    (:`then_1`
      (for _array_element_4 (`self.StoppedCarsMap`)
        (`/Game/Carla/Blueprints/TrafficLight/BP_CustomTriggerComponent.LightTrafficStateChanged` _array_element_4 TrafficLightState)))))

(fn `CreateCarObservers`
  (for _array_element (`self.K2_GetComponentsByClass` "/Script/Engine.BoxComponent")
    (if (not (`KismetStringLibrary.EqualEqual_StrStr` (`KismetSystemLibrary.GetDisplayName` _array_element) "TotalVolume"))
      (bind _returnvalue (`AddComponent|NODE_AddBP_CustomTriggerComponent-0`))
      (`KismetArrayLibrary.Array_Add` (`self.StoppedCarsMap`) _returnvalue)
      (set `/Game/Carla/Blueprints/TrafficLight/BP_CustomTriggerComponent.BoxCollider` _array_element _returnvalue)
      (`/Game/Carla/Blueprints/TrafficLight/BP_CustomTriggerComponent.BindOverlap` _returnvalue))))

(fn `GetTriggerVolume`
  (returns (ReturnValue :type "BoxComponent Object Reference"))
  (return (`self.TotalVolume`)))

(fn `UserConstructionScript`
  (locals (CurrentMaterial :type "MaterialInstanceDynamic Object Reference"))
  (bind _currentmaterial (`local.CurrentMaterial`))
  (bind _currentmaterial_2 (`local.CurrentMaterial`))
  (for _array_element (`self.Heads`)
    (bind (_description _position _lights) (break `/Game/Carla/Static/TrafficLight/Streetlights_01/TrafficLightStructure` _array_element))
    (bind _returnvalue (`AddComponent|NODE_AddStaticMeshComponent-1` :`RelativeTransform` _position))
    (`StaticMeshComponent.SetStaticMesh` _returnvalue "/Game/Carla/Static/TrafficLight/Streetlights_01/SM_TL_BotCover.SM_TL_BotCover")
    (for _array_element_2 _lights
      (bind (_mesh _relativetransform _lightcolor _masked _mask _rotation) (break `/Game/Carla/Static/TrafficLight/Streetlights_01/TrafficLightPieceStructure` _array_element_2))
      (bind _returnvalue_2 (`AddComponent|NODE_AddStaticMeshComponent-2` :`RelativeTransform` _relativetransform))
      (`SceneComponent.K2_AttachToComponent` _returnvalue_2 _returnvalue "None" "KeepRelative" "KeepRelative" "KeepRelative" false)
      (`StaticMeshComponent.SetStaticMesh` _returnvalue_2 _mesh)
      (if _masked
        (bind _returnvalue_3 (`PrimitiveComponent.CreateDynamicMaterialInstance` _returnvalue_2 1 "/Game/Carla/Static/TrafficLight/Streetlights_01/M_StreetlightsMasked.M_StreetlightsMasked" "None"))
        (set `local.CurrentMaterial` _returnvalue_3)
        (else
          (bind _returnvalue_4 (`PrimitiveComponent.CreateDynamicMaterialInstance` _returnvalue_2 1 "/Game/Carla/Static/TrafficLight/Streetlights_01/M_StreetlightsMaster.M_StreetlightsMaster" "None"))
          (set `local.CurrentMaterial` _returnvalue_4)))
      (`MaterialInstanceDynamic.SetTextureParameterValue` _currentmaterial_2 "LightMask" _mask)
      (`MaterialInstanceDynamic.SetScalarParameterValue` _currentmaterial_2 "Angle" _rotation)
      (switch `/Game/Carla/Static/TrafficLight/Streetlights_01/StreetLightColor` _lightcolor
        (:`NewEnumerator0`
          (`MaterialInstanceDynamic.SetVectorParameterValue` _currentmaterial "LightColor" (struct :`R` 30000.0 :`A` 1.0))
          (`KismetArrayLibrary.Array_Add` (`self.RedLights`) _currentmaterial))
        (:`NewEnumerator1`
          (`MaterialInstanceDynamic.SetVectorParameterValue` _currentmaterial "LightColor" (struct :`R` 30000.0 :`G` 20000.0 :`A` 1.0))
          (`KismetArrayLibrary.Array_Add` (`self.YellowLights`) _currentmaterial))
        (:`NewEnumerator2`
          (`MaterialInstanceDynamic.SetVectorParameterValue` _currentmaterial "LightColor" (struct :`G` 30000.0 :`A` 1.0))
          (`KismetArrayLibrary.Array_Add` (`self.GreenLights`) _currentmaterial))))))