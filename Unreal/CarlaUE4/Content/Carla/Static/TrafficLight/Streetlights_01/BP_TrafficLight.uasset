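; BP_TrafficLight is a CARLA traffic light that shows its current state and reports it to wheeled vehicles at the light.
; BoxTrigger overlaps add vehicles to StoppedCars and notify them, then remove and un-notify them on exit.
; On each state change it swaps red, yellow and green lamp materials, setting the lit lamp's On/Off parameter, then re-notifies every tracked vehicle.
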(event `self.BoxTrigger.OnComponentBeginOverlap`
  (params (OverlappedComponent :type "PrimitiveComponent Object Reference") (OtherActor :type "Actor Object Reference") (OtherComp :type "PrimitiveComponent Object Reference") (OtherBodyIndex :type Integer) (bFromSweep :type Boolean) (SweepResult :type "HitResult Structure (by ref)"))
  (bind _ascarla_wheeled_vehicle (cast `CarlaWheeledVehicle` OtherActor))
  (`KismetArrayLibrary.Array_Add` (`self.StoppedCars`) _ascarla_wheeled_vehicle)
  (`self.NotifyWheeledVehicle` _ascarla_wheeled_vehicle))

(event `self.BoxTrigger.OnComponentEndOverlap`
  (params (OverlappedComponent :type "PrimitiveComponent Object Reference") (OtherActor :type "Actor Object Reference") (OtherComp :type "PrimitiveComponent Object Reference") (OtherBodyIndex :type Integer))
  (`/Engine/EditorBlueprintResources/StandardMacros.IsValid` OtherActor
    (:`Is Valid`
      (bind _ascarla_wheeled_vehicle (cast `CarlaWheeledVehicle` OtherActor))
      (`self.UnNotifyWheeledVehicle` _ascarla_wheeled_vehicle)
      (`KismetArrayLibrary.Array_RemoveItem` (`self.StoppedCars`) _ascarla_wheeled_vehicle))))

(event `self.OnTrafficLightStateChanged`
  (params (TrafficLightState :type "TrafficLightState Structure"))
  (bind (_bred _byellow _bgreen) (break `TrafficLightState` TrafficLightState))
  (bind _yellowlight (`self.YellowLight`))
  (bind _greenlight (`self.GreenLight`))
  (bind _redlight (`self.RedLight`))
  (`|ExecutionSequence`
    (:`then_0`
      (if _bred
        _
        (elif _byellow
          _
          (elif (not _bgreen)
            (`PrimitiveComponent.SetMaterial` (`self.RedLight`) 1 "/Game/Carla/Static/TrafficLight/Streetlights_01/MI_StreetLightsOff.MI_StreetLightsOff")
            (`PrimitiveComponent.SetMaterial` (`self.YellowLight`) 1 "/Game/Carla/Static/TrafficLight/Streetlights_01/MI_StreetLightsOff.MI_StreetLightsOff")
            (`PrimitiveComponent.SetMaterial` (`self.GreenLight`) 1 "/Game/Carla/Static/TrafficLight/Streetlights_01/MI_StreetLightsOff.MI_StreetLightsOff")))))
    (:`then_1`
      (if _bred
        (`PrimitiveComponent.SetMaterial` _redlight 1 "/Game/Carla/Static/TrafficLight/Streetlights_01/MI_Streetlights_2.MI_Streetlights_2")
        (`MeshComponent.SetScalarParameterValueOnMaterials` _redlight "On/Off" 1.0)
        (`PrimitiveComponent.SetMaterial` (`self.YellowLight`) 1 "/Game/Carla/Static/TrafficLight/Streetlights_01/MI_StreetLightsOff.MI_StreetLightsOff")
        (`PrimitiveComponent.SetMaterial` (`self.GreenLight`) 1 "/Game/Carla/Static/TrafficLight/Streetlights_01/MI_StreetLightsOff.MI_StreetLightsOff")))
    (:`then_2`
      (if _byellow
        (`PrimitiveComponent.SetMaterial` (`self.RedLight`) 1 "/Game/Carla/Static/TrafficLight/Streetlights_01/MI_StreetLightsOff.MI_StreetLightsOff")
        (`PrimitiveComponent.SetMaterial` _yellowlight 1 "/Game/Carla/Static/TrafficLight/Streetlights_01/MI_Streetlights_1.MI_Streetlights_1")
        (`MeshComponent.SetScalarParameterValueOnMaterials` _yellowlight "On/Off" 1.0)
        (`PrimitiveComponent.SetMaterial` (`self.GreenLight`) 1 "/Game/Carla/Static/TrafficLight/Streetlights_01/MI_StreetLightsOff.MI_StreetLightsOff")))
    (:`then_3`
      (if _bgreen
        (`PrimitiveComponent.SetMaterial` (`self.RedLight`) 1 "/Game/Carla/Static/TrafficLight/Streetlights_01/MI_StreetLightsOff.MI_StreetLightsOff")
        (`PrimitiveComponent.SetMaterial` (`self.YellowLight`) 1 "/Game/Carla/Static/TrafficLight/Streetlights_01/MI_StreetLightsOff.MI_StreetLightsOff")
        (`PrimitiveComponent.SetMaterial` _greenlight 1 "/Game/Carla/Static/TrafficLight/Streetlights_01/MI_Streetlights_3.MI_Streetlights_3")
        (`MeshComponent.SetScalarParameterValueOnMaterials` _greenlight "On/Off" 1.0)))
    (:`then_4`
      (for _array_element (`self.StoppedCars`)
        (`self.NotifyWheeledVehicle` _array_element)))))

(fn `GetTriggerVolume`
  (returns (ReturnValue :type "BoxComponent Object Reference"))
  (return (`self.BoxTrigger`)))

(fn `UserConstructionScript`)