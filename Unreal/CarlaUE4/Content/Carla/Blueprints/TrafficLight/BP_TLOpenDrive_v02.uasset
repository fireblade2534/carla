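; Data-driven CARLA traffic light actor (OpenDrive, v02) that builds its signal heads and switches lamps as its light state changes.
; The construction script spawns support and light meshes from Heads, gives each light a masked or master dynamic material, and sorts those materials by color.
; LightChanged toggles each color group's "On/Off" parameter.
; Construction also occasionally randomizes the Sign mesh from Props, while the exposed BoxTrigger's overlap events are empty.
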(event `TrafficLightInterface.LightChanged`
  (params (NewLightState :type "TrafficLightState Structure"))
  (bind (_bred _byellow _bgreen) (break `TrafficLightState` NewLightState))
  (for _array_element (`self.RedLights`)
    (`MaterialInstanceDynamic.SetScalarParameterValue` _array_element "On/Off" (`KismetMathLibrary.SelectFloat` 1.0 0.0 _bred)))
  (for _array_element_2 (`self.YellowLights`)
    (`MaterialInstanceDynamic.SetScalarParameterValue` _array_element_2 "On/Off" (`KismetMathLibrary.SelectFloat` 1.0 0.0 _byellow)))
  (for _array_element_3 (`self.GreenLights`)
    (`MaterialInstanceDynamic.SetScalarParameterValue` _array_element_3 "On/Off" (`KismetMathLibrary.SelectFloat` 1.0 0.0 _bgreen))))

(event `self.BoxTrigger.OnComponentBeginOverlap`
  (params (OverlappedComponent :type "PrimitiveComponent Object Reference") (OtherActor :type "Actor Object Reference") (OtherComp :type "PrimitiveComponent Object Reference") (OtherBodyIndex :type Integer) (bFromSweep :type Boolean) (SweepResult :type "HitResult Structure (by ref)")))

(event `self.BoxTrigger.OnComponentEndOverlap`
  (params (OverlappedComponent :type "PrimitiveComponent Object Reference") (OtherActor :type "Actor Object Reference") (OtherComp :type "PrimitiveComponent Object Reference") (OtherBodyIndex :type Integer)))

(fn `GetTriggerVolume`
  (returns (ReturnValue :type "BoxComponent Object Reference"))
  (return (`self.BoxTrigger`)))

(fn `UserConstructionScript`
  (locals (CurrentMaterial :type "MaterialInstanceDynamic Object Reference"))
  (bind _props (`self.Props`))
  (bind _currentmaterial (`local.CurrentMaterial`))
  (bind _currentmaterial_2 (`local.CurrentMaterial`))
  (`|ExecutionSequence`
    (:`then_0`
      (for _array_element (`self.Heads`)
        (bind (_description _position _lights _support) (break `/Game/Carla/Blueprints/TrafficLight/ST_TrafficLightHead` _array_element))
        (bind _returnvalue (`AddComponent|NODE_AddStaticMeshComponent-1` :`RelativeTransform` _position))
        (`StaticMeshComponent.SetStaticMesh` _returnvalue _support)
        (for _array_element_2 _lights
          (bind (_mesh _relativetransform _lightcolor _masked _mask _rotation) (break `/Game/Carla/Static/TrafficLight/Streetlights_01/TrafficLightPieceStructure` _array_element_2))
          (bind _returnvalue_2 (`AddComponent|NODE_AddStaticMeshComponent-2` :`RelativeTransform` _relativetransform))
          (`SceneComponent.K2_AttachToComponent` _returnvalue_2 _returnvalue "None" "KeepRelative" "KeepRelative" "KeepRelative" false)
          (`StaticMeshComponent.SetStaticMesh` _returnvalue_2 _mesh)
          (if _masked
            (bind _returnvalue_3 (`PrimitiveComponent.CreateDynamicMaterialInstance` _returnvalue_2 1 "/Game/Carla/Static/TrafficLight/Materials/M_StreetlightsMasked_T10.M_StreetlightsMasked_T10" "None"))
            (set `local.CurrentMaterial` _returnvalue_3)
            (else
              (bind _returnvalue_4 (`PrimitiveComponent.CreateDynamicMaterialInstance` _returnvalue_2 1 "/Game/Carla/Static/TrafficLight/Materials/M_StreetlightsMaster_T10.M_StreetlightsMaster_T10" "None"))
              (set `local.CurrentMaterial` _returnvalue_4)))
          (`MaterialInstanceDynamic.SetTextureParameterValue` _currentmaterial_2 "LightMask" _mask)
          (`MaterialInstanceDynamic.SetScalarParameterValue` _currentmaterial_2 "Angle" _rotation)
          (switch `/Game/Carla/Static/TrafficLight/Streetlights_01/StreetLightColor` _lightcolor
            (:`NewEnumerator0`
              (`MaterialInstanceDynamic.SetVectorParameterValue` _currentmaterial "LightColor" (struct :`R` 1.0 :`G` 0.015686 :`A` 1.0))
              (`KismetArrayLibrary.Array_Add` (`self.RedLights`) _currentmaterial))
            (:`NewEnumerator1`
              (`MaterialInstanceDynamic.SetVectorParameterValue` _currentmaterial "LightColor" (struct :`R` 1.0 :`G` 0.745098 :`A` 1.0))
              (`KismetArrayLibrary.Array_Add` (`self.YellowLights`) _currentmaterial))
            (:`NewEnumerator2`
              (`MaterialInstanceDynamic.SetVectorParameterValue` _currentmaterial "LightColor" (struct :`G` 1.0 :`A` 1.0))
              (`KismetArrayLibrary.Array_Add` (`self.GreenLights`) _currentmaterial)))
          (if (`KismetMathLibrary.RandomBoolWithWeight` 0.1)
            (`StaticMeshComponent.SetStaticMesh` (`self.Sign`) (`|GetArrayItem` _props (`KismetMathLibrary.RandomInteger` (`KismetArrayLibrary.Array_Length` _props))))))))
    (:`then_1`)))